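; BP_WarnLight is a warning spotlight that flashes while the player is fully detected.
; BeginPlay caches the light's original color and the player's SpiderBot pawn.
; LightSwitcher, not called within this Blueprint, re-calls itself after a one-second delay, alternating between the supplied and original colors.
; When the player's game manager no longer reports full detection, it sets the light to white and stops looping.
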(event Custom|LightSwitcher
  (params (c_Color :type Color%20Structure))
  (if (Variables|/Game/BP/GameManager.GameManager_C|Getb_FullyDetected (Variables|/Game/BP/SpiderBot.SpiderBot_C|Getg_GameManager (Variables|Default|GetPlayer)))
    (Rendering|Components|Light|SetLightColor (Variables|Default|GetSpotLight) (Math|Conversions|ToLinearColor(Color) c_Color) true)
    (if (Variables|Default|Getb_LightSwitched)
      (Variables|Default|Setc_NewColor (stale _output_get))
      (else
        (bind _output_get (Variables|Default|Setc_ChosenColor c_Color))
        (Variables|Default|Setc_NewColor (Variables|Default|Getc_OldColor))))
    (Variables|Default|Setb_LightSwitched (not (Variables|Default|Getb_LightSwitched)))
    (Utilities|FlowControl|Delay 1.0)
    (CallFunction|LightSwitcher (Variables|Default|Getc_NewColor))
    (else
      (Rendering|Components|Light|SetLightColor (Variables|Default|GetSpotLight) "(R=1.000000,G=1.000000,B=1.000000,A=1.000000)" true))))

(event EventBeginPlay
  (Variables|Default|Setc_OldColor (Math|Conversions|ToColor(LinearColor) (Rendering|Components|Light|GetLightColor (Variables|Default|GetSpotLight))))
  (bind _asspider_bot (Utilities|Casting|CastToSpiderBot (Game|Player|GetPlayerPawn 0)))
  (Variables|Default|SetPlayer _asspider_bot))

(fn ConstructionScript)