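; BP_Screw is a screw that can be screwed in once, reporting to a parent object when done.
; Each external GettingScrewed call, while the screw is unfinished, sets its timer to DeltaTime minus the stored time, a reversed operand order for a countdown.
; A result at or below zero marks it screwed and increments the parent's screw-hit count.
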(event Custom|GettingScrewed
  (params (DeltaTime :type Float%20%28single-precision%29))
  (if (not (Variables|Default|Getb_IsScrewed))
    (Variables|Default|Setf_ScrewTime (- DeltaTime (Variables|Default|Getf_ScrewTime)))
    (if (<= (Variables|Default|Getf_ScrewTime) 0.0)
      (Variables|Default|Setb_IsScrewed true)
      (Variables|/Game/BP/BP_ScrewParent.BP_ScrewParent_C|Seti_ScrewsHit (Variables|Default|Getg_Parent) (+ (Variables|/Game/BP/BP_ScrewParent.BP_ScrewParent_C|Geti_ScrewsHit (Variables|Default|Getg_Parent)) 1)))))

(fn ConstructionScript)